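; BP_SplinePlacement is a construction-time placement tool that repeats a chosen static mesh at regular intervals along a spline.
; The construction script assigns the mesh to an InstancedStaticMesh component, then adds instances using the spline's local-space location and rotation at each spacing step.
; CalculateNumberOfInstances supplies the loop bound, with its graph dividing spline length by spacing and rounding down.
; The event graph has no active runtime logic.
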(fn `UserConstructionScript`
  (bind _spline (`self.Spline`))
  (`StaticMeshComponent.SetStaticMesh` (`self.InstancedStaticMesh`) (`self.StaticMeshVar`))
  (for _index (range (+ (`self.CalculateNumberOfInstances`) 1))
    (bind _returnvalue (* _index (`self.SpaceBetweenInstances`)))
    (`InstancedStaticMeshComponent.AddInstance` (`self.InstancedStaticMesh`) (`KismetMathLibrary.MakeTransform` (`SplineComponent.GetLocationAtDistanceAlongSpline` _spline _returnvalue "Local") (`SplineComponent.GetRotationAtDistanceAlongSpline` _spline _returnvalue "Local")) false)))