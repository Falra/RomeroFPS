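; BP_EnemySpawner is a spawner actor that keeps enemy characters populating the level up to a maximum count.
; On BeginPlay it starts a looping timer that counts all BP_EnemyCharacter actors in the world.
; When the count is below MaxEnemies, SpawnEnemy spawns one with BT_EnemyBehavior at a random navigable point within a large radius around the spawner.
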(event `self.ReceiveBeginPlay`
  (`KismetSystemLibrary.K2_SetTimerDelegate` (delegate `TrySpawnEnemy`) (`self.SpawnTime`) true))

(event `TrySpawnEnemy`
  ;[1 1 1] Spawn Enemies
  (bind _outactors (`GameplayStatics.GetAllActorsOfClass` "/Game/Romero/Enemy/BP_EnemyCharacter.BP_EnemyCharacter_C"))
  (if (< (`KismetArrayLibrary.Array_Length` _outactors) (`self.MaxEnemies`))
    (`self.SpawnEnemy`)))

(fn `UserConstructionScript`)