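; BP_CollectionsTest is a scratch Blueprint that lays out collection nodes for testing and has no runtime behavior.
; Its event graph holds unconnected array operations on AmmoSet, which is an array despite its name, and set operations on UniqueNames.
; These cover edits, queries, conversion and set algebra, but no event reaches them, and the construction script is empty.
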(fn `UserConstructionScript`)