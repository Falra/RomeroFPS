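; BP_CylinderTarget is a moving shooting target that takes two projectile hits to destroy.
; A looping timer reverses its direction, and Tick moves it along that normalized direction at a set speed, scaled by delta time.
; The first BP_FirstPersonProjectile hit turns it red and primes it.
; The next plays explosion effects, increments the player's TargetsEliminated count, calls CheckGoal and destroys the target.
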(event `self.ReceiveBeginPlay`
  ;[1 1 1] Change direction on timer
  (`KismetSystemLibrary.K2_SetTimerDelegate` (delegate `ChangeDirection`) (`self.TimeToChange`) true))

(event `ChangeDirection`
  ;[1 1 1] Change direction on timer
  (set `self.Direction` (* (`self.Direction`) -1.0)))

(event `self.ReceiveTick`
  (params (DeltaSeconds :type "Float (single-precision)"))
  ;[1 1 1] Update location every frame
  (`self.K2_AddActorWorldOffset` (* (`KismetMathLibrary.Normal` (`self.Direction`)) (* (`GameplayStatics.GetWorldDeltaSeconds`) (`self.Speed`)))))

(event `self.ReceiveHit`
  (params (MyComp :type "PrimitiveComponent Object Reference") (Other :type "Actor Object Reference") (OtherComp :type "PrimitiveComponent Object Reference") (bSelfMoved :type Boolean) (HitLocation :type "Vector Structure") (HitNormal :type "Vector Structure") (NormalImpulse :type "Vector Structure") (Hit :type "HitResult Structure (by ref)"))
  ;[1 1 1] On hit: first turn red, then explode
  (cast `/Game/FirstPerson/Blueprints/BP_FirstPersonProjectile` Other)
  (if (`self.Primed`)
    (`GameplayStatics.PlaySoundAtLocation` "/Game/StarterContent/Audio/Explosion01.Explosion01" HitLocation (struct) 1.0 1.0 0.0 null null null null)
    (`GameplayStatics.SpawnEmitterAtLocation` "/Game/StarterContent/Particles/P_Explosion.P_Explosion" HitLocation)
    (bind _asbp_first_person_character (cast `/Game/FirstPerson/Blueprints/BP_FirstPersonCharacter` (`GameplayStatics.GetPlayerCharacter` 0)))
    (`/Engine/EditorBlueprintResources/StandardMacros.IncrementInt` (`/Game/FirstPerson/Blueprints/BP_FirstPersonCharacter.TargetsEliminated` _asbp_first_person_character)
      (:`  `
        (`/Game/FirstPerson/Blueprints/BP_FirstPersonCharacter.CheckGoal` _asbp_first_person_character)
        (`self.K2_DestroyActor`)))
    (else
      (`PrimitiveComponent.SetMaterial` (`self.StaticMeshComponent`) 0 "/Game/Romero/Materials/MM_TargetRed.MM_TargetRed")
      (set `self.Primed` true))))

(fn `UserConstructionScript`)