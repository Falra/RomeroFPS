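; BP_DiceLibrary is a dice-rolling function library with functions for one, two or three dice of a given face count.
; Each rolls random integers from 1 to the face count, and the multi-die versions return the sum and individual dice.
; The three-die function stores rolls in variables before summing, while the two-die function wires random calls straight into its outputs.
; Face counts of 1 or less print an error message.
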(fn `RoolOneDie`
  (params (NumberOfFaces :type Integer :default 6))
  (returns (Result :type Integer))
  (if (> NumberOfFaces 1)
    (return (`KismetMathLibrary.RandomIntegerInRange` 1 NumberOfFaces))
    (else
      (`KismetSystemLibrary.PrintString` null "Number of Faces must be greater than 1"))))

(fn `RoolThreeDies`
  (params (NumberOfFaces :type Integer :default 6))
  (returns (Sum :type Integer) (Die1 :type Integer) (Die2 :type Integer) (Die3 :type Integer))
  (locals (Die1Var :type Integer) (Die2Var :type Integer) (Die3Var :type Integer))
  (bind _returnvalue (`KismetMathLibrary.RandomIntegerInRange` 1 NumberOfFaces))
  (bind _die1var (`local.Die1Var`))
  (bind _die2var (`local.Die2Var`))
  (bind _die3var (`local.Die3Var`))
  (if (> NumberOfFaces 1)
    (set `local.Die1Var` _returnvalue)
    (set `local.Die2Var` _returnvalue)
    (set `local.Die3Var` _returnvalue)
    (return (+ _die1var _die2var _die3var) _die1var _die2var _die3var)
    (else
      (`KismetSystemLibrary.PrintString` null "Number of Faces must be greater than 1"))))

(fn `RoolTwoDies`
  (params (NumberOfFaces :type Integer :default 6))
  (returns (Sum :type Integer) (Die1 :type Integer) (Die2 :type Integer))
  (bind _returnvalue (`KismetMathLibrary.RandomIntegerInRange` 1 NumberOfFaces))
  (bind _returnvalue_2 (`KismetMathLibrary.RandomIntegerInRange` 1 NumberOfFaces))
  (if (> NumberOfFaces 1)
    (return (+ _returnvalue _returnvalue_2) _returnvalue _returnvalue_2)
    (else
      (`KismetSystemLibrary.PrintString` null "Number of Faces must be greater than 1"))))